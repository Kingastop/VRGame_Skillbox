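; VR catapult actor that is wound by a gripped wheel and fired by a linked physics button.
; Tick converts accumulated wheel rotation into the Spring constraint's angular target, lowering the arm until fully cocked and then enabling the LoadHandle's drives.
; Once cocked, a sphere trace finds a CatapultProjectile and attaches it with physics off.
; Pressing the button detaches the projectile, restores physics and swings the spring target back to launch it.
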(event Custom|ReleasedSpring
  (Transformation|DetachFromActor (Variables|Default|GetProjectile) "KeepRelative" "KeepRelative" "KeepRelative")
  (Transformation|SetActorLocation (Variables|Default|GetProjectile) (Math|Vector|MakeVector (.x (Transformation|GetActorLocation (Variables|Default|GetProjectile))) (.y (Transformation|GetActorLocation (Variables|Default|GetProjectile))) (+ (.z (Transformation|GetActorLocation (Variables|Default|GetProjectile))) (/ (.z (Transformation|GetActorScale3D (Variables|Default|GetProjectile))) 2.0))) false true)
  (Physics|SetSimulatePhysics (Variables|/Game/DesktopVRMain/Blueprints/CatapultProjectile.CatapultProjectile_C|GetSphere (Variables|Default|GetProjectile)) true)
  (Class|PhysicsConstraintComponent|SetAngularOrientationTarget (Variables|Default|GetSpring) (Math|Rotator|MakeRotator 0.0 45.0 0.0))
  (Class|PrimitiveComponent|WakeRigidBody (Variables|Default|Getcatapult_arm) "None")
  (CallFunction|Reseter)
  (CallFunction|ResetBtn)
  (Utilities|FlowControl|Delay 2.0)
  (Variables|Default|SetProjectile 0)
  (Variables|Default|SetProjectileLoaded? false))

(event Custom|ButtonPressed
  (params (FoundedButton :type Physics%20Button%20Object%20Reference))
  (EventDispatchers|BindEventtoOnPressed FoundedButton (delegate Custom|FoundedButton)))

(event Custom|Loading
  (params (MotionController :type Motion%20Controller%20Component%20Object%20Reference))
  (Variables|Default|SetWheelMoving? true)
  (Variables|Default|SetPreviousAngle 0.0)
  (Variables|Default|SetArmAngle 0.0)
  (Variables|Default|SetWheelAngle 0.0)
  (Class|PhysicsConstraintComponent|SetOrientationDriveTwistandSwing (Variables|Default|GetLoadHandle) false false))

(event Custom|Reseter
  (Utilities|FlowControl|DoOnce false) ; enters at Reset
)

(event Custom|FoundedButton
  (CallFunction|ReleasedSpring))

(event Custom|ResetBtn
  (Utilities|FlowControl|DoOnce false) ; enters at Reset
)

(event EventBeginPlay
  (Transformation|SetWorldRotation (Variables|Default|Getcatapult_arm) (Math|Transform|TransformRotation (Transformation|GetActorTransform) "0, 0, 0") false false)
  (EventDispatchers|BindEventtoOnGrip (Variables|Default|GetPhysics_Grip_component) (delegate Custom|Loading))
  (bind _asphysics_button (Utilities|Casting|CastToPhysicsButton (Variables|Default|GetChosenLauncher)))
  (Rendering|Material|SetMaterial (Variables|/Game/DesktopVRMain/Blueprints/PhysicsButton.PhysicsButton_C|GetCylinder _asphysics_button) 0 (Utilities|Array|Get(acopy) (Rendering|Material|GetMaterials (Variables|Default|Getcatapult_base))))
  (bind _output_get (Variables|Default|SetAs%20Physics%20Button _asphysics_button))
  (Utilities|IsValid _output_get
    (:Is%20Valid
      (CallFunction|ButtonPressed (Variables|Default|GetAs%20Physics%20Button)))))

(event EventTick
  (params (DeltaSeconds :type Float%20%28single-precision%29))
  (bind _physics_grip_component1 (Variables|Default|GetPhysics_Grip_component1))
  (bind _as_physics_button (Variables|Default|GetAs%20Physics%20Button))
  (bind _returnvalue (Transformation|GetWorldLocation _physics_grip_component1))
  (Utilities|FlowControl|Delay 1.0)
  (Utilities|FlowControl|Sequence
    (:then_0
      (if (Variables|Default|GetWheelMoving?)
        (bind _output_get (Variables|Default|SetCurrentAngle (.pitch (Variables|/Script/Engine.SceneComponent|GetRelativeRotation (Variables|Default|GetLoadWheel)))))
        (bind _output_get_2 (Variables|Default|SetWheelAngle (+ (Variables|Default|GetWheelAngle) (Math|Float|Absolute(Float) (- _output_get (Variables|Default|GetPreviousAngle))))))
        (bind _output_get_3 (Variables|Default|SetArmAngle (- 45.0 (/ _output_get_2 8.0))))
        (if (> _output_get_3 -45.0)
          (Class|PhysicsConstraintComponent|SetAngularOrientationTarget (Variables|Default|GetSpring) (Math|Rotator|MakeRotator 0.0 _output_get_3 0.0))
          (Class|PrimitiveComponent|WakeRigidBody (Variables|Default|Getcatapult_arm) "None")
          (else
            (Variables|Default|SetArmAngle -45.0)
            (Class|PhysicsConstraintComponent|SetAngularOrientationTarget (Variables|Default|GetSpring) (Math|Rotator|MakeRotator 0.0 -45.0 0.0))
            (Variables|Default|SetWheelMoving? false)
            (Utilities|FlowControl|DoOnce false
              (:Completed
                (Class|PhysicsConstraintComponent|SetOrientationDriveTwistandSwing (Variables|Default|GetLoadHandle) true true)
                (Class|PhysicsConstraintComponent|SetAngularOrientationTarget (Variables|Default|GetLoadHandle) (Math|Rotator|MakeRotator 0.0 0.0 0.0))
                (Class|PrimitiveComponent|WakeRigidBody (Variables|Default|GetLoadWheel) "None")))))
        (else
          (Utilities|FlowControl|Sequence
            (:then_0
              (if (and (<= (Variables|Default|GetArmAngle) -45.0) (not (Variables|Default|GetProjectileLoaded?)))
                (bind _outhit (Collision|SphereTraceForObjects _returnvalue _returnvalue 5e+01 (Utilities|Array|MakeArray "ObjectTypeQuery4") false 0 "Persistent" true "(R=0.000000,G=1.000000,B=1.000000,A=1.000000)" "(R=0.000000,G=1.000000,B=0.000000,A=1.000000)" 1.0))
                (bind _ascatapult_projectile (Utilities|Casting|CastToCatapultProjectile (.HitActor (Collision|BreakHitResult _outhit))))
                (bind _output_get_4 (Variables|Default|SetProjectile _ascatapult_projectile))
                (Transformation|AttachActorToActor _output_get_4 (Components|GetOwner (Variables|Default|Getcatapult_arm)) "None" "KeepRelative" "KeepRelative" "KeepRelative" true)
                (Physics|SetSimulatePhysics (Variables|/Game/DesktopVRMain/Blueprints/CatapultProjectile.CatapultProjectile_C|GetSphere _output_get_4) false)
                (Transformation|SetActorRelativeLocation _output_get_4 (Variables|/Script/Engine.SceneComponent|GetRelativeLocation (Variables|Default|GetPhysics_Grip_component1)) false true)
                (Variables|Default|SetProjectileLoaded? true)))
            (:then_1
              (if (and (Variables|/Game/DesktopVRMain/Blueprints/PhysicsButton.PhysicsButton_C|GetPressed? _as_physics_button) (<= (Variables|Default|GetArmAngle) -45.0))
                (Utilities|FlowControl|DoOnce false
                  (:Completed
                    (CallFunction|ButtonPressed _as_physics_button)))))))))
    (:then_1
      (Variables|Default|SetPreviousAngle (Variables|Default|GetCurrentAngle)))))

(fn ConstructionScript)