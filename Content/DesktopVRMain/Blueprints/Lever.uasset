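; Physics-driven lever with a grippable handle that settles toward one of two sides in the DesktopVR project.
; When the PhysicsGripComponent drops it, the sign of the handle's roll sets LeverSwitch, defaulting to positive at zero.
; That value drives the PhysicsConstraint's angular velocity and orientation targets.
; RemoteSwitch sets the same targets from a supplied destination and wakes the handle's rigid body.
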(event Custom|LeverSwitched
  (bind _physicsconstraint (Variables|Default|GetPhysicsConstraint))
  (bind _handle (Variables|Default|GetHandle))
  (bind _relativerotation (Variables|/Script/Engine.SceneComponent|GetRelativeRotation _handle))
  (bind _returnvalue (Math|Float|Absolute(Float) (.roll _relativerotation)))
  (bind _returnvalue_2 (/ (.roll _relativerotation) _returnvalue))
  (if (== _returnvalue_2 0.0)
    (Variables|Default|SetLeverSwitch 1.0)
    (else
      (Variables|Default|SetLeverSwitch _returnvalue_2)))
  (Class|PhysicsConstraintComponent|SetAngularVelocityTarget _physicsconstraint (Math|Vector|MakeVector (Variables|Default|GetLeverSwitch) 0.0 0.0))
  (Class|PhysicsConstraintComponent|SetAngularOrientationTarget _physicsconstraint (Math|Rotator|MakeRotator (Variables|Default|GetLeverSwitch) 0.0 0.0)))

(event Custom|RemoteSwitch
  (params (Destination :type Float%20%28single-precision%29))
  (bind _physicsconstraint (Variables|Default|GetPhysicsConstraint))
  (bind _output_get (Variables|Default|SetLeverSwitch Destination))
  (Class|PhysicsConstraintComponent|SetAngularVelocityTarget _physicsconstraint (Math|Vector|MakeVector _output_get 0.0 0.0))
  (Class|PhysicsConstraintComponent|SetAngularOrientationTarget _physicsconstraint (Math|Rotator|MakeRotator _output_get 0.0 0.0))
  (Class|PrimitiveComponent|WakeRigidBody (Variables|Default|GetHandle) "None"))

(event EventBeginPlay
  (EventDispatchers|AssignOnDrop (Variables|Default|GetPhysics_Grip_component) (delegate Custom|LeverSwitched)))

(event Collision|EventActorBeginOverlap
  (params (OtherActor :type Actor%20Object%20Reference)))

(event EventTick
  (params (DeltaSeconds :type Float%20%28single-precision%29)))

(fn ConstructionScript)