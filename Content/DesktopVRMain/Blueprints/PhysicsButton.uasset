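; PhysicsButton is a physical push button, in a desktop VR project, that fires an OnPressed event when its cube is pushed down.
; A physics constraint limits vertical travel, and BeginPlay sets the press threshold half that limit below the cube's starting world Z.
; Tick, gated by a one-second Delay, compares the cube's relative Z to that threshold.
; A DoOnce, reset on release, limits each press to one event and records the frame delta as PressTime.
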(event Custom|BtnReleased
  (Variables|Default|SetPressed? false)
  (CallFunction|Reseter))

(event Custom|BtnPressed
  (Variables|Default|SetPressed? true)
  (Utilities|FlowControl|DoOnce false
    (:Completed
      (Variables|Default|SetPressTime (Variables|Default|GetDelta%20Seconds))
      (Default|CallOnPressed))))

(event Custom|Reseter
  (Utilities|FlowControl|DoOnce false) ; enters at Reset
)

(event EventBeginPlay
  (Class|PhysicsConstraintComponent|SetLinearZLimit (Variables|Default|GetPhysicsConstraint) "LCM_Limited" (Variables|Default|GetLimit))
  (Variables|Default|SetPressedLocation (- (.z (Transformation|GetWorldLocation (Variables|Default|GetCube))) (/ (Variables|Default|GetLimit) 2.0))))

(event EventTick
  (params (DeltaSeconds :type Float%20%28single-precision%29))
  (Variables|Default|SetDelta%20Seconds DeltaSeconds)
  (Utilities|FlowControl|Delay 1.0)
  (if (<= (.z (Variables|/Script/Engine.SceneComponent|GetRelativeLocation (Variables|Default|GetCube))) (Variables|Default|GetPressedLocation))
    (CallFunction|BtnPressed)
    (elif (Variables|Default|GetPressed?)
      (CallFunction|BtnReleased))))

(fn ConstructionScript)