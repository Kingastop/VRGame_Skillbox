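; VR TV actor that plays a media playlist as channels, switched by linked next and previous button actors.
; It saves each channel's playback time in an array and seeks back to it after a one-second delay when reopening.
; A trigger box resumes playback when the VR character enters and pauses and saves the time on exit, using DoOnce gates reset by each handler.
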(event OnComponentBeginOverlap(Box)
  (params (OverlappedComponent :type Primitive%20Component%20Object%20Reference) (OtherActor :type Actor%20Object%20Reference) (OtherComp :type Primitive%20Component%20Object%20Reference) (OtherBodyIndex :type Integer) (bFromSweep :type Boolean) (SweepResult :type Hit%20Result%20Structure%20%28by%20ref%29))
  (Utilities|Casting|CastToVRCharacter OtherActor)
  (Variables|Default|SetWatching? true)
  (Utilities|FlowControl|DoOnce false
    (:Completed
      (CallFunction|VideoPlay (Variables|Default|GetNowPlayingIndex)))))

(event OnComponentEndOverlap(Box)
  (params (OverlappedComponent :type Primitive%20Component%20Object%20Reference) (OtherActor :type Actor%20Object%20Reference) (OtherComp :type Primitive%20Component%20Object%20Reference) (OtherBodyIndex :type Integer))
  (Utilities|Casting|CastToVRCharacter OtherActor)
  (Variables|Default|SetWatching? false)
  (Utilities|FlowControl|DoOnce false
    (:Completed
      (CallFunction|VideoPause))))

(event Custom|OpenVideo
  (params (SourceIndex :type Integer) (Watch :type Boolean))
  (bind _mediaplayer (Variables|Default|GetMediaPlayer))
  (Sequencer|Player|Pause (Variables|Default|GetMediaPlayer))
  (Utilities|FlowControl|Delay 1.0)
  (bind _output_get (Variables|Default|SetNowPlayingIndex SourceIndex))
  (Variables|/Script/MediaAssets.MediaPlayer|SetPlayOnOpen _mediaplayer Watch)
  (Media|MediaPlayer|Seek _mediaplayer (Utilities|Array|Get(acopy) (Variables|Default|GetTimeStopped) _output_get))
  (Development|PrintString (Utilities|String|Append (Utilities|String|ToString(Integer) (.Seconds (Math|Timespan|BreakTimespan (Utilities|Array|Get(acopy) (Variables|Default|GetTimeStopped) _output_get)))) "    " (Utilities|String|ToString(Integer) _output_get)) true true "(R=0.000000,G=0.660000,B=1.000000,A=1.000000)" 1e+02)
  (Media|MediaPlayer|Play _mediaplayer :!class /Script/MediaAssets.MediaPlayer))

(event Custom|SaveTime
  (bind _mediaplayer (Variables|Default|GetMediaPlayer))
  (Sequencer|Player|Pause _mediaplayer)
  (Utilities|Array|SetArrayElem (Variables|Default|GetTimeStopped) (Variables|/Script/MediaAssets.MediaPlayer|GetPlaylistIndex _mediaplayer) (Class|MediaPlayer|GetTime _mediaplayer)))

(event Custom|PreviousChannel
  (bind _nowplayingindex (Variables|Default|GetNowPlayingIndex))
  (bind _mediaplayer (Variables|Default|GetMediaPlayer))
  (bind _returnvalue (- _nowplayingindex 1))
  (bind _playlist (Variables|/Script/MediaAssets.MediaPlayer|GetPlaylist _mediaplayer))
  (CallFunction|SaveTime)
  (if (> _returnvalue 0)
    (Variables|Default|SetNextTrack _returnvalue)
    (else
      (bind _returnvalue_2 (Class|MediaPlaylist|Num _playlist))
      (Variables|Default|SetNextTrack (- _returnvalue_2 1))))
  (Sequencer|Player|Pause _mediaplayer)
  (Class|MediaPlayer|OpenPlaylistIndex _mediaplayer _playlist (Variables|Default|GetNextTrack))
  (CallFunction|OpenVideo (Variables|Default|GetNextTrack) true))

(event Custom|VideoPlay
  (params (Index :type Integer))
  (CallFunction|OpenVideo Index true)
  (CallFunction|OnPause))

(event Custom|NextChannel
  (bind _nowplayingindex (Variables|Default|GetNowPlayingIndex))
  (bind _mediaplayer (Variables|Default|GetMediaPlayer))
  (bind _returnvalue (+ _nowplayingindex 1))
  (bind _playlist (Variables|/Script/MediaAssets.MediaPlayer|GetPlaylist _mediaplayer))
  (CallFunction|SaveTime)
  (bind _returnvalue_2 (Class|MediaPlaylist|Num _playlist))
  (if (< _returnvalue _returnvalue_2)
    (Variables|Default|SetNextTrack _returnvalue)
    (else
      (Variables|Default|SetNextTrack 0)))
  (Sequencer|Player|Pause _mediaplayer)
  (Class|MediaPlayer|OpenPlaylistIndex _mediaplayer _playlist (Variables|Default|GetNextTrack))
  (CallFunction|OpenVideo (Variables|Default|GetNextTrack) true))

(event Custom|VideoPause
  (bind _mediaplayer (Variables|Default|GetMediaPlayer))
  (bind _playlistindex (Variables|/Script/MediaAssets.MediaPlayer|GetPlaylistIndex _mediaplayer))
  (Sequencer|Player|Pause _mediaplayer)
  (Utilities|Array|SetArrayElem (Variables|Default|GetTimeStopped) _playlistindex (Class|MediaPlayer|GetTime _mediaplayer))
  (Variables|Default|SetNowPlayingIndex _playlistindex)
  (CallFunction|OnStart))

(event Custom|OnStart
  (Utilities|FlowControl|DoOnce false) ; enters at Reset
)

(event Custom|OnPause
  (Utilities|FlowControl|DoOnce false) ; enters at Reset
)

(event EventBeginPlay
  (bind _buttonnext (Variables|Default|GetButtonNext))
  (bind _buttonprevious (Variables|Default|GetButtonPrevious))
  (bind _cube (Variables|Default|GetCube))
  (bind _mplaylist (Variables|Default|GetMPlaylist))
  (bind _mediaplayer (Variables|Default|GetMediaPlayer))
  (bind _returnvalue (Rendering|Material|GetMaterials _cube))
  (bind _output (Utilities|Array|Get(acopy) _returnvalue))
  (Class|MediaPlayer|OpenPlaylist (Variables|Default|GetMediaPlayer) (Variables|Default|GetMPlaylist))
  (bind _returnvalue_2 (Class|MediaPlaylist|Num _mplaylist))
  (for _index (range 0 (- _returnvalue_2 1))
    (bind _returnvalue_3 (Utilities|Array|Get(acopy) _mplaylist _index))
    (Utilities|Array|Add (Variables|Default|GetSources) _returnvalue_3)
    (Utilities|Array|Add (Variables|Default|GetTimeStopped) (Variables|Default|GetZeros)))
  (if (and (Utilities|IsValid (Variables|Default|GetButtonNext)) (Utilities|IsValid (Variables|Default|GetButtonPrevious)))
    (EventDispatchers|BindEventtoOnPressed (Variables|Default|GetButtonNext) (delegate Custom|NextChannel))
    (EventDispatchers|BindEventtoOnPressed (Variables|Default|GetButtonPrevious) (delegate Custom|PreviousChannel))
    (Rendering|Material|SetMaterial (Variables|/Game/DesktopVRMain/Blueprints/PhysicsButton.PhysicsButton_C|GetCube _buttonnext) 0 "/Engine/TemplateResources/MI_Template_BaseBlue.MI_Template_BaseBlue")
    (Rendering|Material|SetMaterial (Variables|/Game/DesktopVRMain/Blueprints/PhysicsButton.PhysicsButton_C|GetCylinder _buttonnext) 0 _output)
    (Rendering|Material|SetMaterial (Variables|/Game/DesktopVRMain/Blueprints/PhysicsButton.PhysicsButton_C|GetCylinder _buttonprevious) 0 _output)
    (Rendering|Material|SetMaterial (Variables|/Game/DesktopVRMain/Blueprints/PhysicsButton.PhysicsButton_C|GetCube _buttonprevious) 0 "/Game/DesktopVRMain/Models/PB_Catapult_Models/HandleMaterial.HandleMaterial")
    (Class|MediaPlayer|OpenPlaylistIndex _mediaplayer (Variables|/Script/MediaAssets.MediaPlayer|GetPlaylist _mediaplayer))
    (CallFunction|OpenVideo 0 (Variables|Default|GetWatching?))))

(fn ConstructionScript)