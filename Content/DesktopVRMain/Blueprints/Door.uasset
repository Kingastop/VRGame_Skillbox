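; Physics-driven door with a knob that toggles the latch and re-locks automatically, built on physics constraints.
; Tick, throttled by Delays, compares knob roll to its BeginPlay value: near it, the door's swing unlocks and the knob's twist locks; otherwise the door stays locked.
; Once toggled, AutoLock waits until the door yaw returns near its starting angle, then locks the swing and resets the knob and its constraint.
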(event Custom|DoorLock
  (Class|PhysicsConstraintComponent|SetAngularSwing1Limit (Variables|Default|GetOpenDoor) "ACM_Locked" 0.0))

(event Custom|AutoLock
  (bind _doorgrip (Variables|Default|GetDoorGrip))
  (bind _lockedrotation (Variables|Default|GetLockedRotation))
  (bind _returnvalue (Transformation|GetWorldRotation _doorgrip))
  (bind _returnvalue_2 (- (.yaw _returnvalue) _lockedrotation))
  (bind _returnvalue_3 (Math|Float|Absolute(Float) _returnvalue_2))
  (if (and (<= _returnvalue_3 1e+01) (>= _returnvalue_3 0.0))
    (Variables|Default|SetToggled? false)
    (CallFunction|DoorLock)
    (Transformation|SetWorldRotation (Variables|Default|GetKnob) (Math|Transform|TransformRotation (Transformation|GetActorTransform) "0, 0, 0") false false)
    (Class|PhysicsConstraintComponent|SetAngularTwistLimit (Variables|Default|GetToggleHandle) "ACM_Limited" 3e+01)
    (Class|PhysicsConstraintComponent|SetAngularOrientationTarget (Variables|Default|GetToggleHandle) (Math|Rotator|MakeRotator 3e+01 0.0 0.0))
    (Class|PrimitiveComponent|WakeRigidBody (Variables|Default|GetKnob) "None")
    (Utilities|FlowControl|Delay 5.0)))

(event EventBeginPlay
  (Variables|Default|SetLockedRotation (.yaw (Transformation|GetWorldRotation (Variables|Default|GetDoorGrip))))
  (Variables|Default|SetKnobRotation (.roll (Transformation|GetWorldRotation (Variables|Default|GetKnob)))))

(event Collision|EventActorBeginOverlap
  (params (OtherActor :type Actor%20Object%20Reference)))

(event EventTick
  (params (DeltaSeconds :type Float%20%28single-precision%29))
  (bind _knobrotation (Variables|Default|GetKnobRotation))
  (bind _knob (Variables|Default|GetKnob))
  (bind _returnvalue (Transformation|GetWorldRotation _knob))
  (bind _returnvalue_2 (- (.roll _returnvalue) _knobrotation))
  (bind _returnvalue_3 (Math|Float|Absolute(Float) _returnvalue_2))
  (Utilities|FlowControl|Delay 1.0)
  (if (Variables|Default|GetToggled?)
    (Utilities|FlowControl|Delay 4.0)
    (CallFunction|AutoLock)
    (elif (and (<= _returnvalue_3 1e+01) (>= _returnvalue_3 0.0))
      (Variables|Default|SetToggled? true)
      (Class|PhysicsConstraintComponent|SetAngularOrientationTarget (Variables|Default|GetToggleHandle) (Math|Rotator|MakeRotator -3e+01 0.0 0.0))
      (Class|PrimitiveComponent|WakeRigidBody (Variables|Default|GetKnob) "None")
      (Class|PhysicsConstraintComponent|SetAngularTwistLimit (Variables|Default|GetToggleHandle) "ACM_Locked" 0.0)
      (Class|PhysicsConstraintComponent|SetAngularSwing1Limit (Variables|Default|GetOpenDoor) "ACM_Limited" 1e+02)
      (else
        (CallFunction|DoorLock)))))

(fn ConstructionScript)