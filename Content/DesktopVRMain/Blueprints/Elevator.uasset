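; VR elevator actor that travels vertically between Basement and FirstFloor heights, controlled by an attached lever or linked physics buttons.
; BeginPlay collects buttons from ChosenLauncher and binds the lever's grip-drop event to ElevatorMove.
; While idle, Tick tracks the most recently pressed button, whose height remotely flips the lever toward the nearer floor.
; The lever state sets the Delta sign, and Tick offsets the root until clamped at either limit.
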(event Custom|LeverPulled
  (CallFunction|ElevatorMove))

(event Custom|ButtonPressed
  (params (FoundedButton :type Physics%20Button%20Object%20Reference))
  (EventDispatchers|BindEventtoOnPressed FoundedButton (delegate Custom|FoundedButton)))

(event Custom|ElevatorMove
  (bind _thisbutton (Variables|Default|GetThisButton))
  (bind _firstfloor (Variables|Default|GetFirstFloor))
  (bind _elevatorlever (Variables|Default|GetElevatorLever))
  (bind _returnvalue (Transformation|GetActorLocation _thisbutton))
  (bind _returnvalue_2 (- (.z _returnvalue) _firstfloor))
  (bind _returnvalue_3 (Math|Float|Absolute(Float) _returnvalue_2))
  (if (Utilities|IsValid _thisbutton)
    (Development|PrintString "Hello")
    (if (== _returnvalue_3 (Math|Float|Min(Float) _returnvalue_3 (Math|Float|Absolute(Float) (- (.z _returnvalue) (Variables|Default|GetBasement)))))
      (Default|RemoteSwitch _elevatorlever 1.0)
      (else
        (Default|RemoteSwitch _elevatorlever -1.0)))
    (Variables|Default|SetDelta (* (Variables|/Game/DesktopVRMain/Blueprints/Lever.Lever_C|GetLeverSwitch (Variables|Default|GetElevatorLever)) (Math|Float|Absolute(Float) (Variables|Default|GetDelta))))
    (Variables|Default|SetMoving? true)
    (CallFunction|Reseter)
    (else
      (Utilities|IsValid (Variables|Default|GetElevatorLever)
        (:Is%20Valid
          (Development|PrintString (Utilities|String|ToString(Float) (* (Variables|/Game/DesktopVRMain/Blueprints/Lever.Lever_C|GetLeverSwitch (Variables|Default|GetElevatorLever)) (Math|Float|Absolute(Float) (Variables|Default|GetDelta)))))
          (Variables|Default|SetDelta (* (Variables|/Game/DesktopVRMain/Blueprints/Lever.Lever_C|GetLeverSwitch (Variables|Default|GetElevatorLever)) (Math|Float|Absolute(Float) (Variables|Default|GetDelta))))
          (Variables|Default|SetMoving? true)
          (CallFunction|Reseter))))))

(event Custom|Reseter
  (Utilities|FlowControl|DoOnce false) ; enters at Reset
)

(event Custom|FoundedButton
  (CallFunction|ElevatorMove))

(event Custom|ResetBtn
  (Utilities|FlowControl|DoOnce false) ; enters at Reset
)

(event EventBeginPlay
  (for _array_element (Variables|Default|GetChosenLauncher)
    (bind _asphysics_button (Utilities|Casting|CastToPhysicsButton _array_element))
    (Rendering|Material|SetMaterial (Variables|/Game/DesktopVRMain/Blueprints/PhysicsButton.PhysicsButton_C|GetCylinder _asphysics_button) 0 (Utilities|Array|Get(acopy) (Rendering|Material|GetMaterials (Variables|Default|GetCube1))))
    (Utilities|Array|Add (Variables|Default|GetButtons) _asphysics_button))
  (for _array_element_2 (Actor|GetAttachedActors true)
    (bind _aslever (Utilities|Casting|CastToLever _array_element_2))
    (bind _output_get (Variables|Default|SetElevatorLever _aslever)))
  (Utilities|IsValid (Variables|Default|GetElevatorLever)
    (:Is%20Valid
      (EventDispatchers|BindEventtoOnDrop (Variables|/Game/DesktopVRMain/Blueprints/Lever.Lever_C|GetPhysics_Grip_component _output_get) (delegate Custom|LeverPulled)))))

(event EventTick
  (params (DeltaSeconds :type Float%20%28single-precision%29))
  (bind _returnvalue (Transformation|GetActorLocation))
  (bind _returnvalue_2 (Transformation|GetActorLocation))
  (bind _returnvalue_3 (Transformation|GetActorLocation))
  (bind _defaultsceneroot (Variables|Default|GetDefaultSceneRoot))
  (if (Variables|Default|GetMoving?)
    (Utilities|FlowControl|Sequence
      (:then_0
        (Utilities|FlowControl|DoOnce false
          (:Completed
            (Variables|Default|SetMoving? false)
            (Utilities|FlowControl|Delay 2.0)
            (Variables|Default|SetMoving? true))))
      (:then_1
        (Transformation|AddWorldOffset (Variables|Default|GetDefaultSceneRoot) (Math|Vector|MakeVector 0.0 0.0 (Variables|Default|GetDelta)) false false)
        (Utilities|FlowControl|Sequence
          (:then_0
            (if (> (.z _returnvalue) (Variables|Default|GetFirstFloor))
              (Transformation|SetWorldLocation _defaultsceneroot (Math|Vector|MakeVector (.x _returnvalue_2) (.y _returnvalue_2) (Variables|Default|GetFirstFloor)) false false)
              (Variables|Default|SetMoving? false)
              (CallFunction|ResetBtn)))
          (:then_1
            (if (> (Variables|Default|GetBasement) (.z _returnvalue))
              (Transformation|SetWorldLocation _defaultsceneroot (Math|Vector|MakeVector (.x _returnvalue_3) (.y _returnvalue_3) (Variables|Default|GetBasement)) false false)
              (Variables|Default|SetMoving? false)
              (CallFunction|ResetBtn))))))
    (elif (> (Utilities|Array|Length (Variables|Default|GetButtons)) 0)
      (for _array_element (Variables|Default|GetButtons)
        (if (Variables|/Game/DesktopVRMain/Blueprints/PhysicsButton.PhysicsButton_C|GetPressed? _array_element)
          (Utilities|IsValid (Variables|Default|GetThisButton)
            (:Is%20Valid
              (if (> (Variables|/Game/DesktopVRMain/Blueprints/PhysicsButton.PhysicsButton_C|GetPressTime _array_element) (Variables|/Game/DesktopVRMain/Blueprints/PhysicsButton.PhysicsButton_C|GetPressTime (Variables|Default|GetThisButton)))
                (Variables|Default|SetThisButton _array_element)))
            (:Is%20Not%20Valid
              (Variables|Default|SetThisButton _array_element)))))
      (Utilities|IsValid (Variables|Default|GetThisButton)
        (:Is%20Valid
          (Utilities|FlowControl|DoOnce false
            (:Completed
              (CallFunction|ButtonPressed (Variables|Default|GetThisButton)))))))))

(fn ConstructionScript)